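; AttackLine is an attack actor that turns toward a target and stretches into a line, using the GameManager's top or bottom side material.
; StartAttack launches it at boosted speed, which decays to its initial speed while Tick adds speed-scaled length to the root's X scale every frame.
; Growth stops once the projected tip leaves the GameManager boundary plus leeway.
; Tip sphere-overlap and hitbox hit handling only print debug strings.
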(event OnComponentHit(Hitbox)
  (params (HitComponent :type Primitive%20Component%20Object%20Reference) (OtherActor :type Actor%20Object%20Reference) (OtherComp :type Primitive%20Component%20Object%20Reference) (NormalImpulse :type Vector :default "0, 0, 0") (Hit :type Hit%20Result%20Structure%20%28by%20ref%29))
  (Development|PrintString (Utilities|String|Append (Utilities|GetDisplayName self) (Utilities|GetDisplayName OtherActor))))

(event EventBeginPlay)

(event Collision|EventActorBeginOverlap
  (params (OtherActor :type Actor%20Object%20Reference)))

(event EventTick
  (params (DeltaSeconds :type Float%20%28single-precision%29))
  (bind _returnvalue (Transformation|GetActorRotation))
  (bind _returnvalue_2 (Transformation|GetActorLocation))
  (bind _boundaryleeway (Variables|Default|GetBoundaryLeeway))
  (bind _defaultsceneroot (Variables|Default|GetDefaultSceneRoot))
  (bind _visuals (Variables|Default|GetVisuals))
  (bind _boundaryleeway_2 (Variables|Default|GetBoundaryLeeway))
  (bind _returnvalue_3 (Math|Vector|GetForwardVector _returnvalue))
  (bind _returnvalue_4 (Transformation|GetWorldScale _defaultsceneroot))
  (bind (_min _max) (Components|StaticMesh|GetLocalBounds _visuals))
  (bind _returnvalue_5 (Transformation|GetWorldScale _visuals))
  (bind _x (Math|Vector|BreakVector _max))
  (bind (_x_2 _y _z) (Math|Vector|BreakVector _returnvalue_4))
  (bind _x_3 (Math|Vector|BreakVector _returnvalue_5))
  (bind _x_4 (Math|Vector|BreakVector _min))
  (bind _returnvalue_6 (- _x _x_4))
  (bind _returnvalue_7 (* _x_3 _returnvalue_6))
  (bind _returnvalue_8 (* _returnvalue_3 _returnvalue_7))
  (bind _returnvalue_9 (+ _returnvalue_2 _returnvalue_8))
  (bind (_x_5 _y_2) (Math|Vector|BreakVector _returnvalue_9))
  (if (Variables|Default|GetActivated)
    (Variables|Default|SetSpeed (Math|Float|Clamp(Float) (- (Variables|Default|GetSpeed) (* DeltaSeconds (* (Variables|Default|GetBoostFrictionRate) (Variables|Default|GetSpeed)))) (Variables|Default|GetInitialSpeed) 99999.0))
    (Transformation|SetWorldScale3D _defaultsceneroot (Math|Vector|MakeVector (+ _x_2 (* (Math|Float|Clamp(Float) (- (Variables|Default|GetSpeed) (* DeltaSeconds (* (Variables|Default|GetBoostFrictionRate) (Variables|Default|GetSpeed)))) (Variables|Default|GetInitialSpeed) 99999.0) (Variables|Default|GetSpeedToScale))) _y _z))
    (bind _asgame_manager (Utilities|Casting|CastToGameManager (Game|GetGameInstance)))
    ;[1 1 1] If the extended point of cube is within screen boundaries
    (bind (_width _height) (Default|GetBoundary _asgame_manager))
    (if (and (Math|Float|InRange(Float) _x_5 (- (* (/ _height 2.0) -1.0) _boundaryleeway_2) (+ (/ _height 2.0) _boundaryleeway_2) false false) (Math|Float|InRange(Float) _y_2 (- (* (/ _width 2.0) -1.0) _boundaryleeway) (+ (/ _width 2.0) _boundaryleeway) false false))
      (bind (_outactors _returnvalue_10) (Collision|SphereOverlapActors _returnvalue_9 0.0 (Utilities|Array|MakeArray "ObjectTypeQuery7") "AttackLine_C"))
      (if _returnvalue_10
        (if (not (== (stale _array_element) self))
          (Development|PrintString "Hello")))
      (else
        (Variables|Default|SetActivated false)))))

(fn ConstructionScript)

(fn StartAttack
  (params (TargetLocation :type Vector) (Speed :type Float%20%28single-precision%29))
  (bind _output_get (Variables|Default|SetInitialSpeed Speed))
  (Variables|Default|SetSpeed (* _output_get (Variables|Default|GetSpeedBoostMultiplier)))
  (Transformation|SetActorRotation (Math|Rotator|FindLookatRotation (Transformation|GetActorLocation) TargetLocation))
  (Variables|Default|SetActivated true)
  (Rendering|SetActorHiddenInGame false))

(fn SetInitialParameters
  (params (TopSide :type Boolean))
  (bind _visuals (Variables|Default|GetVisuals))
  (bind _output_get (Variables|Default|SetTopSide TopSide))
  (bind _asgame_manager (Utilities|Casting|CastToGameManager (Game|GetGameInstance)))
  (if _output_get
    (Rendering|Material|SetMaterial _visuals 0 (Variables|/Game/Blueprints/GameManager.GameManager_C|GetTopMaterial _asgame_manager))
    (else
      (Rendering|Material|SetMaterial _visuals 0 (Variables|/Game/Blueprints/GameManager.GameManager_C|GetBotMaterial _asgame_manager)))))