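; LineRules runs the two-sided touch play field, fitting colored top and bottom areas to the orthographic camera and storing bounds in GameManager.
; Touches inside either area spawn a blue or red spline, tracked per finger.
; Releasing after enough drag launches that spline, with speed based on drag distance.
; Each launch adds camera shake and a hit-stop via global time dilation, both scaled by drag, with Tick restoring normal time.
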(event `self.ReceiveBeginPlay`
  (bind _toparea (`self.TopArea`))
  (bind _botarea (`self.BotArea`))
  (bind _z (.z (`self.K2_GetActorLocation` (`self.BotArea`))))
  (bind (_boundarywidth _boundaryheight) (`self.SetBoundaryVariables`))
  (`self.SetAreaToScale` _toparea _boundarywidth _boundaryheight)
  (bind _x (`self.GetBoundaryActorX`))
  (`self.K2_SetActorLocation` _toparea (`KismetMathLibrary.MakeVector` _x 0.0 _z) false true)
  (`self.SetAreaToScale` _botarea _boundarywidth _boundaryheight)
  (`self.K2_SetActorLocation` _botarea (`KismetMathLibrary.MakeVector` (* _x -1.0) 0.0 _z) false true)
  (bind _asgame_manager (cast `/Game/Blueprints/GameManager` (`GameplayStatics.GetGameInstance`)))
  (`self.Set Bound Color` (`/Game/Blueprints/FieldBoundaries.Cube` (`self.TopArea`)) (`KismetMathLibrary.Conv_ColorToLinearColor` (`/Game/Blueprints/GameManager.TopColor` _asgame_manager)))
  (`self.Set Bound Color` (`/Game/Blueprints/FieldBoundaries.Cube` (`self.BotArea`)) (`KismetMathLibrary.Conv_ColorToLinearColor` (`/Game/Blueprints/GameManager.BotColor` _asgame_manager))))

(event `InputTouch`
  (params (Location :type "Vector Structure") (FingerIndex :type "ETouchIndex Enum"))
  (bind _returnvalue (`KismetMathLibrary.Conv_ByteToInt` FingerIndex))
  (bind _returnvalue_2 (`KismetMathLibrary.Conv_ByteToInt` FingerIndex))
  (bind _activespline (`self.ActiveSpline`))
  (bind _maxtouchdistance (`self.MaxTouchDistance`))
  (bind _activespline_2 (`self.ActiveSpline`))
  (bind _timedilationspeed (`self.TimeDilationSpeed`))
  (bind _returnvalue_3 (`KismetMathLibrary.Vector_Distance` Location (`|GetArrayItem` (`self.TouchArray`) _returnvalue_2)))
  (bind _returnvalue_4 (`KismetMathLibrary.FClamp` _returnvalue_3 0.0 _maxtouchdistance))
  (:`Pressed`
    (`KismetArrayLibrary.Array_Insert` (`self.TouchArray`) Location _returnvalue)
    (bind _placementworldlocation (`self.TouchVectorToPlacement` Location))
    (bind _x (`self.GetBoundaryAreaX`))
    (bind _x_2 (.x _placementworldlocation))
    (if (not (`KismetMathLibrary.InRange_FloatFloat` _x_2 (* _x -1.0) _x false false))
      (bind _returnvalue_5 (> _x_2 0.0))
      (if _returnvalue_5
        (bind _returnvalue_6 (`KismetMathLibrary.Conv_VectorToTransform` _placementworldlocation))
        (bind _returnvalue_7 (`|SpawnActorFromClass` "/Game/Blueprints/SplineBlue.SplineBlue_C" _returnvalue_6 "Undefined" "OverrideRootScale" null null))
        (`KismetArrayLibrary.Array_Insert` _activespline _returnvalue_7 _returnvalue)
        (else
          (bind _returnvalue_8 (`|SpawnActorFromClass` "/Game/Blueprints/SplineRed.SplineRed_C" _returnvalue_6 "Undefined" "OverrideRootScale" null null))
          (`KismetArrayLibrary.Array_Insert` _activespline _returnvalue_8 _returnvalue)))
      (`/Game/Blueprints/Spline.SetInitalParameters` _returnvalue_7 _returnvalue_5)
      (`/Game/Blueprints/Spline.SetInitalParameters` _returnvalue_7 _returnvalue_5)))
  (:`Released`
    (if (`KismetArrayLibrary.Array_IsValidIndex` (`self.ActiveSpline`) _returnvalue_2)
      (if (>= _returnvalue_3 (`self.MinTouchDistance`))
        (set `self.EffectScale` (/ _returnvalue_4 _maxtouchdistance))
        (bind _placementworldlocation_2 (`self.TouchVectorToPlacement` Location))
        (`/Game/Blueprints/Spline.Set Attack Parameters` (`|GetArrayItem` _activespline_2 _returnvalue_2) _placementworldlocation_2 (+ (* _returnvalue_4 (`self.TouchDistanceToSpeed`)) (`self.SplineSpeedBoost`)))
        (`KismetArrayLibrary.Array_Remove` _activespline_2 _returnvalue_2)
        (`PlayerCameraManager.StartCameraShake` :`self` (`GameplayStatics.GetPlayerCameraManager` 0) :`ShakeClass` "/Game/Blueprints/CameraShake.CameraShake_C" :`Scale` (`self.EffectScale`))
        ;[1 1 1] HitStop Code
        (`GameplayStatics.SetGlobalTimeDilation` _timedilationspeed)
        (set `self.HitStopTimer` (* _timedilationspeed (`self.HitStopDuration`) (`self.EffectScale`)))
        (set `self.HitStopActive` true)))))

(event `self.ReceiveTick`
  (params (DeltaSeconds :type "Float (single-precision)"))
  ;[1 1 1] HitStop Code
  (if (>= DeltaSeconds (`self.TimeDilationSpeed`))
    _
    (elif (`self.HitStopActive`)
      (set `self.HitStopTimer` (- (`self.HitStopTimer`) (`GameplayStatics.GetWorldDeltaSeconds`)))
      (if (<= (`self.HitStopTimer`) 0.0)
        (set `self.HitStopActive` false)
        (`GameplayStatics.SetGlobalTimeDilation` 1.0)))))

(fn `GetBoundaryActorX`
  (returns (X :type "Float (double-precision)"))
  (return (- (/ (`self.BoundaryHeight`) 2.0) (/ (* (`self.BoundaryHeight`) (`self.TouchAreaProportion`)) 2.0))))

(fn `GetBoundaryAreaX`
  (returns (X :type "Float (double-precision)"))
  (return (- (/ (`self.BoundaryHeight`) 2.0) (* (`self.BoundaryHeight`) (`self.TouchAreaProportion`)))))

(fn `Set Bound Color`
  (params (Object :type "PrimitiveComponent Object Reference") (Color :type "LinearColor Structure"))
  (bind _returnvalue (`PrimitiveComponent.CreateDynamicMaterialInstance` Object 0 null "None"))
  (`MaterialInstanceDynamic.SetVectorParameterValue` _returnvalue "Color" Color))

(fn `SetAreaToScale`
  (params (Boundary :type "/Game/Blueprints/FieldBoundaries Object Reference") (Width :type "Float (double-precision)") (Height :type "Float (double-precision)"))
  (bind (_min _max) (`StaticMeshComponent.GetLocalBounds` (`/Game/Blueprints/FieldBoundaries.Cube` Boundary)))
  (`self.SetActorScale3D` Boundary (`KismetMathLibrary.MakeVector` (* (/ Height (.x (- _max _min))) (`self.TouchAreaProportion`)) (/ Width (.y (- _max _min))) (.z (`self.GetActorScale3D` Boundary)))))

(fn `SetBoundaryVariables`
  (returns (BoundaryWidth :type "Float (double-precision)") (BoundaryHeight :type "Float (double-precision)"))
  (bind _ascamera_actor (cast `CameraActor` (`self.CameraActor`)))
  (bind _cameracomponent (`CameraActor.CameraComponent` _ascamera_actor))
  (bind _orthowidth (`CameraComponent.OrthoWidth` _cameracomponent))
  (bind _output_get (set `self.BoundaryWidth` _orthowidth))
  (bind _output_get_2 (set `self.BoundaryHeight` (/ _orthowidth (`CameraComponent.AspectRatio` _cameracomponent))))
  (bind _asgame_manager (cast `/Game/Blueprints/GameManager` (`GameplayStatics.GetGameInstance`)))
  (`/Game/Blueprints/GameManager.SetBoundary` _asgame_manager _output_get _output_get_2)
  (return _output_get _output_get_2))

(fn `TouchVectorToPlacement`
  (params (ScreenLocation :type "Vector Structure"))
  (returns (PlacementWorldLocation :type "Vector Structure"))
  (bind (_returnvalue_x _returnvalue_y _returnvalue_z) (`KismetMathLibrary.BreakVector` (`self.K2_GetActorLocation` (`self.PlacementLayer`))))
  (return (`KismetMathLibrary.MakeVector` (.x (`PlayerController.DeprojectScreenPositionToWorld` (`GameplayStatics.GetPlayerController` 0) (.x ScreenLocation) (.y ScreenLocation))) (.y (`PlayerController.DeprojectScreenPositionToWorld` (`GameplayStatics.GetPlayerController` 0) (.x ScreenLocation) (.y ScreenLocation))) _returnvalue_z)))

(fn `UserConstructionScript`
  (`self.SetBoundaryVariables`))