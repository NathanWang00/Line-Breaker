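; Spline actor for an attack that, once activated, stretches its last point toward a target direction until it leaves the GameManager boundary.
; The construction script builds spline mesh segments between points, and SetInitalParameters picks a top or bottom material.
; SetAttackParameters sets boosted speed and direction, then Tick applies clamped friction, extends the spline and refits the meshes.
; Tick also rebinds segment overlaps, whose handler only prints the other actor's name.
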(event `CustomEvent_2`
  (params (OverlappedComponent :type "PrimitiveComponent Object Reference") (OtherActor :type "Actor Object Reference") (OtherComp :type "PrimitiveComponent Object Reference") (OtherBodyIndex :type Integer) (bFromSweep :type Boolean) (SweepResult :type "HitResult Structure (by ref)"))
  (`KismetSystemLibrary.PrintString` (`KismetSystemLibrary.GetDisplayName` OtherActor)))

(event `CustomEvent_4` :!signature `self.OnActorBeginOverlap`
  (params (OverlappedActor :type "Actor Object Reference") (OtherActor :type "Actor Object Reference"))
  (`KismetSystemLibrary.PrintString` (`KismetSystemLibrary.GetDisplayName` OtherActor)))

(event `self.ReceiveBeginPlay`
  (`self.ClearExtraMesh`))

(event `CustomEvent_3`
  (params (HitComponent :type "PrimitiveComponent Object Reference") (OtherActor :type "Actor Object Reference") (OtherComp :type "PrimitiveComponent Object Reference") (NormalImpulse :type "Vector Structure") (Hit :type "HitResult Structure (by ref)"))
  (`KismetSystemLibrary.PrintString` (`KismetSystemLibrary.GetDisplayName` OtherActor)))

(event `CustomEvent_0` :!signature `self.OnActorBeginOverlap`
  (params (OverlappedActor :type "Actor Object Reference") (OtherActor :type "Actor Object Reference"))
  (`KismetSystemLibrary.PrintString` (`KismetSystemLibrary.GetDisplayName` OtherActor)))

(event `CustomEvent_1` :!signature `self.OnActorHit`
  (params (SelfActor :type "Actor Object Reference") (OtherActor :type "Actor Object Reference") (NormalImpulse :type "Vector Structure") (Hit :type "HitResult Structure (by ref)"))
  (`KismetSystemLibrary.PrintString` (`KismetSystemLibrary.GetDisplayName` OtherActor) :!label _label))

(event `CustomEvent`
  (params (HitComponent :type "PrimitiveComponent Object Reference") (OtherActor :type "Actor Object Reference") (OtherComp :type "PrimitiveComponent Object Reference") (NormalImpulse :type "Vector Structure") (Hit :type "HitResult Structure (by ref)"))
  (goto _label))

(event `self.ReceiveTick`
  (params (DeltaSeconds :type "Float (single-precision)"))
  (bind _spline (`self.Spline`))
  (bind _returnvalue (`KismetMathLibrary.FClamp` (- (`self.Speed`) (* DeltaSeconds (* (`self.BoostFrictionRate`) (`self.Speed`)))) (`self.OriginalSpeed`) 99999.0))
  (if (`self.Activated`)
    (set `self.Speed` _returnvalue)
    (`self.SetExtensionNode` (* DeltaSeconds _returnvalue))
    (for _index (range (+ (- (`SplineComponent.GetNumberOfSplinePoints` (`self.Spline`)) 2) 1))
      (bind _output (`|GetArrayItem` (`self.SplineMeshArray`) _index))
      (`/Engine/EditorBlueprintResources/StandardMacros.IsValid` _output
        (:`Is Valid`
          (`SplineMeshComponent.SetForwardAxis` _output "Y" true)
          (bind (_location _tangent) (`SplineComponent.GetLocationAndTangentAtSplinePoint` _spline _index "Local"))
          (bind (_location_2 _tangent_2) (`SplineComponent.GetLocationAndTangentAtSplinePoint` _spline (+ _index 1) "Local"))
          (`SplineMeshComponent.SetStartAndEnd` _output _location _tangent _location_2 _tangent_2 true)
          (for _array_element (`self.SplineMeshArray`)
            (set `PrimitiveComponent.bGenerateOverlapEvents` true _array_element)
            (add `PrimitiveComponent.OnComponentBeginOverlap` _array_element (delegate `CustomEvent_2`))))))))

(event `self.Spline.OnComponentHit`
  (params (HitComponent :type "PrimitiveComponent Object Reference") (OtherActor :type "Actor Object Reference") (OtherComp :type "PrimitiveComponent Object Reference") (NormalImpulse :type "Vector Structure") (Hit :type "HitResult Structure (by ref)"))
  (`KismetSystemLibrary.PrintString` "Hello"))

(event `self.Spline.OnComponentBeginOverlap`
  (params (OverlappedComponent :type "PrimitiveComponent Object Reference") (OtherActor :type "Actor Object Reference") (OtherComp :type "PrimitiveComponent Object Reference") (OtherBodyIndex :type Integer) (bFromSweep :type Boolean) (SweepResult :type "HitResult Structure (by ref)"))
  (`KismetSystemLibrary.PrintString` (`KismetSystemLibrary.GetDisplayName` OtherActor)))

(fn `AddSplineMesh`
  (bind _spline (`self.Spline`))
  (for _index (range (+ (- (`SplineComponent.GetNumberOfSplinePoints` (`self.Spline`)) 2) 1))
    (bind _returnvalue (`AddComponent|NODE_AddSplineMeshComponent-2`))
    (`PrimitiveComponent.SetMaterial` _returnvalue 0 (`self.Material`))
    (`PrimitiveComponent.SetCollisionEnabled` _returnvalue "QueryAndPhysics")
    (`SplineMeshComponent.SetForwardAxis` _returnvalue "Y" true)
    (bind (_location _tangent) (`SplineComponent.GetLocationAndTangentAtSplinePoint` _spline _index "Local"))
    (bind (_location_2 _tangent_2) (`SplineComponent.GetLocationAndTangentAtSplinePoint` _spline (+ _index 1) "Local"))
    (`SplineMeshComponent.SetStartAndEnd` _returnvalue _location _tangent _location_2 _tangent_2 true)
    (`KismetArrayLibrary.Array_Add` (`self.SplineMeshArray`) _returnvalue))
  (while (> (`KismetArrayLibrary.Array_Length` (`self.SplineMeshArray`)) (- (`SplineComponent.GetNumberOfSplinePoints` (`self.Spline`)) 1))
    (`KismetArrayLibrary.Array_Remove` (`self.SplineMeshArray`))))

(fn `ClearExtraMesh`
  (while (> (`KismetArrayLibrary.Array_Length` (`self.SplineMeshArray`)) (- (`SplineComponent.GetNumberOfSplinePoints` (`self.Spline`)) 1))
    (`KismetArrayLibrary.Array_Remove` (`self.SplineMeshArray`))))

(fn `GetWithinBounds`
  (params (X :type "Float (double-precision)") (Y :type "Float (double-precision)"))
  (returns (Within :type Boolean))
  (bind _asgame_manager (cast `/Game/Blueprints/GameManager` (`GameplayStatics.GetGameInstance`)))
  (bind (_width _height) (`/Game/Blueprints/GameManager.GetBoundary` _asgame_manager))
  (return (and (>= (/ _width 2.0) (`KismetMathLibrary.Abs` Y)) (>= (/ _height 2.0) (`KismetMathLibrary.Abs` X)))))

(fn `Set Attack Parameters`
  (params (Location :type "Vector Structure") (Speed :type "Float (double-precision)"))
  (set `self.Speed` (* Speed (`self.SpeedBoostMultiplier`)))
  (set `self.OriginalSpeed` Speed)
  (set `self.Direction` (`KismetMathLibrary.Normal` (- Location (`SplineComponent.GetLocationAtSplinePoint` (`self.Spline`) 0 "World"))))
  (set `self.Activated` true))

(fn `SetExtensionNode`
  (params (Speed :type "Float (double-precision)"))
  (returns (InBounds :type Boolean))
  (bind _spline (`self.Spline`))
  (bind _returnvalue (- (`SplineComponent.GetNumberOfSplinePoints` _spline) 1))
  (bind _returnvalue_2 (`SplineComponent.GetLocationAtSplinePoint` _spline _returnvalue "World"))
  (bind _within (`self.GetWithinBounds` (.x _returnvalue_2) (.y _returnvalue_2)))
  (if _within
    (`SplineComponent.SetLocationAtSplinePoint` _spline _returnvalue (+ _returnvalue_2 (* (`self.Direction`) Speed)) "World" true)
    (else
      (set `self.Activated` false)))
  (return _within))

(fn `SetInitalParameters`
  (params (Top :type Boolean))
  (bind _output_get (set `self.TopSide` Top))
  (bind _asgame_manager (cast `/Game/Blueprints/GameManager` (`GameplayStatics.GetGameInstance`)))
  (if _output_get
    (set `self.Material` (`/Game/Blueprints/GameManager.TopMaterial` _asgame_manager))
    (else
      (set `self.Material` (`/Game/Blueprints/GameManager.BotMaterial` _asgame_manager)))))

(fn `UserConstructionScript`
  (`self.AddSplineMesh`)
  (`self.ClearExtraMesh`))