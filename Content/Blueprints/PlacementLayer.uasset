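; PlacementLayer is an unfinished actor Blueprint that experiments with camera view math.
; Each tick it casts MainCamera to a CameraActor and prints the tangent of half its field of view as debug output.
; The construction script resets actor scale to one.
; Disconnected nodes for camera height difference, aspect ratio, viewport size and screen deprojection remain unused, so no placement logic runs.
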(event `self.ReceiveTick`
  (params (DeltaSeconds :type "Float (single-precision)"))
  (bind _ascamera_actor (cast `CameraActor` (`self.MainCamera`)))
  (`KismetSystemLibrary.PrintString` (`KismetStringLibrary.Conv_DoubleToString` (`KismetMathLibrary.DegTan` (* (`CameraComponent.FieldOfView` (`CameraActor.CameraComponent` _ascamera_actor)) 0.5)))))

(fn `UserConstructionScript`
  (`self.SetActorScale3D` (1.0 1.0 1.0)))